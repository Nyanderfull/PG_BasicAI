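; Basic enemy AI that acts as a turret, turning toward a first-person player it sees and firing projectiles.
; PawnSensing stores the seen character as the target; Tick smoothly rotates toward it and drops it beyond a range limit.
; While targeting, a Delay-gated flag paces projectiles spawned at the Projectile component and launched along DogPlush's forward vector.
; Movement nodes are unconnected, so it never chases.
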(event `self.ReceiveTick`
  (params (DeltaSeconds :type "Float (single-precision)"))
  (if (`self.Target`)
    (`|ExecutionSequence`
      (:`then_0`
        (`self.K2_SetActorRotation` (`KismetMathLibrary.RLerp` (`self.K2_GetActorRotation`) (`KismetMathLibrary.FindLookAtRotation` (`self.K2_GetActorLocation`) (`self.K2_GetActorLocation` (`self.As BP First Person Character`))) 0.1 true))
        (if (> (`KismetMathLibrary.Vector_Distance` (`self.K2_GetActorLocation`) (`self.K2_GetActorLocation` (`self.As BP First Person Character`))) 1500.0)
          (set `self.Target` false)
          (set `self.As BP First Person Character` null)))
      (:`then_1`
        (if (`self.Spawn Projectile`)
          (bind _returnvalue (`|SpawnActorFromClass` "/Game/FirstPerson/Blueprints/BP_FirstPersonProjectile.BP_FirstPersonProjectile_C" (`SceneComponent.K2_GetComponentToWorld` (`self.Projectile`)) "Undefined" "MultiplyWithRoot" null null))
          (`PrimitiveComponent.AddImpulse` (`/Game/FirstPerson/Blueprints/BP_FirstPersonProjectile.Sphere` _returnvalue) (* (`SceneComponent.GetForwardVector` (`self.dog_plush`)) (`self.Force`)) "None" true)
          (set `self.Spawn Projectile` false)
          (`KismetSystemLibrary.Delay` 0.2)
          (set `self.Spawn Projectile` true))))))

(event `self.PawnSensing.OnSeePawn`
  (params (Pawn :type "Pawn Object Reference"))
  (bind _asbp_first_person_character (cast `/Game/FirstPerson/Blueprints/BP_FirstPersonCharacter` Pawn))
  (set `self.Target` true)
  (set `self.As BP First Person Character` _asbp_first_person_character))

(fn `UserConstructionScript`)